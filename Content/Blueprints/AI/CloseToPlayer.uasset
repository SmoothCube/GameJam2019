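; CloseToPlayer is a Behavior Tree decorator condition for enemy AI that checks the distance between the enemy and its follow target.
; It casts the owner to BP_EnemyController and measures from the controlled pawn to the actor in the TargetToFollow blackboard key.
; Despite the name, it passes when that distance is at least MinDistanceToPlayer, so it is true when the enemy is not close.
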(fn `PerformConditionCheck`
  (params (OwnerActor :type "Actor Object Reference"))
  (returns (ReturnValue :type Boolean))
  (bind _asbp_enemy_controller (cast `/Game/Blueprints/BP_EnemyController` OwnerActor))
  (return (>= (`KismetMathLibrary.VSize` (- (`Actor.K2_GetActorLocation` (`BTFunctionLibrary.GetBlackboardValueAsActor` (`self.TargetToFollow`))) (`Actor.K2_GetActorLocation` (`Controller.K2_GetPawn` _asbp_enemy_controller)))) (`self.MinDistanceToPlayer`))))