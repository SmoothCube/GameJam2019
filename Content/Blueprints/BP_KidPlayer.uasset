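; BP_KidPlayer is the kid player Blueprint, handling HUD, music switching and gun/stick visuals.
; BeginPlay sets game-only input and hides the arm and stick, while ToggleGunMeshes shows the gun and hides the stick.
; ViewHud creates the player HUD and sets audio component activation, ChangeSong swaps dogfight and rolling songs, and Tick caches the gun's muzzle location.
; On destruction, it opens the pause HUD with UI-only input and a visible cursor.
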(event `Change Song`
  (if (not (`AudioComponent.IsPlaying` (`self.DogFightSong`)))
    (`AudioComponent.Play` (`self.DogFightSong`) 0.0)
    (`AudioComponent.Stop` (`self.RolingSang`))
    (else
      (`AudioComponent.Stop` (`self.DogFightSong`))
      (`AudioComponent.Play` (`self.RolingSang`) 0.0))))

(event `ViewHud`
  (bind _returnvalue (`|CreateWidget` "/Game/UI/PlayerHUD.PlayerHUD_C"))
  (`UserWidget.AddToViewport` _returnvalue 0)
  (`ActorComponent.Activate` (`self.DogFightSong`) false)
  (`ActorComponent.Deactivate` (`self.RolingSang`)))

(event `self.ReceiveBeginPlay`
  (`WidgetBlueprintLibrary.SetInputMode_GameOnly` (`GameplayStatics.GetPlayerController` 0))
  (`SceneComponent.SetVisibility` (`self.Arm`) false true)
  (`SceneComponent.SetVisibility` (`self.StickMesh`) false true))

(event `self.ReceiveTick`
  (params (DeltaSeconds :type "Float (single-precision)"))
  (set `self.MuzzleLocation` (`SceneComponent.GetSocketLocation` (`self.GunMesh`) "Muzzle")))

(event `self.ReceiveDestroyed`
  (bind _returnvalue (`GameplayStatics.GetPlayerController` 0))
  (bind _returnvalue_2 (`|CreateWidget` "/Game/UI/PauseHUD.PauseHUD_C"))
  (`UserWidget.AddToViewport` _returnvalue_2 0)
  (`WidgetBlueprintLibrary.SetInputMode_UIOnlyEx` _returnvalue null)
  (set `PlayerController.bShowMouseCursor` true _returnvalue))

(fn `ToggleGunMeshes`
  (`SceneComponent.SetVisibility` (`self.GunMesh`) true false)
  (`SceneComponent.SetVisibility` (`self.StickMesh`) false true))

(fn `UserConstructionScript`)