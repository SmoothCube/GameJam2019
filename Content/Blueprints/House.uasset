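; House Blueprint with a door that closes behind the kid player when the house is flagged as the player's.
; On BeginPlay a player house starts with its door rotated 90 degrees.
; When BP_KidPlayer leaves the Box trigger, a debug message prints and the RotateDoor timeline drives the door's yaw.
; Each timeline update also sets IsDoorClosed and shifts the trigger 2000 units down, preventing retriggering.
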(event `self.ReceiveBeginPlay`
  (if (`self.bIsPlayerHouse`)
    (`SceneComponent.K2_SetRelativeRotation` (`self.door`) (struct :`Yaw` 90.0) false false)))

(event `self.Box.OnComponentEndOverlap`
  (params (OverlappedComponent :type "PrimitiveComponent Object Reference") (OtherActor :type "Actor Object Reference") (OtherComp :type "PrimitiveComponent Object Reference") (OtherBodyIndex :type Integer))
  (if (`self.bIsDoorClosed`)
    _
    (elif (and (`.bSuccess` (cast `/Game/Blueprints/BP_KidPlayer` OtherActor :!pure true)) (`self.bIsPlayerHouse`))
      (`KismetSystemLibrary.PrintString` "LukkerDør")
      (bind (_direction _rotate) (`Timeline|RotateDoor` :!via `PlayFromStart`)
        (:`Update`
          (`SceneComponent.K2_SetRelativeRotation` (`self.door`) (`KismetMathLibrary.MakeRotator` 0.0 0.0 _rotate) false false)
          (set `self.bIsDoorClosed` true)
          (`SceneComponent.K2_AddLocalOffset` (`self.Box`) (0.0 0.0 -2000.0) false true))))))

(fn `UserConstructionScript`)